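; Player controller for the multiplayer lobby that manages each player's lobby UI and chat.
; Its events create the Lobby widget with server details, update its player list and count, and swap it for a loading screen.
; Chat messages are tagged with the player's name and relayed through LobbyGameMode's AllPCs to each controller's chat window.
; Kick opens the Menu level and destroys the session, while AssignPlayer is an empty stub.
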(event Custom|AddLobbyWB
  (params (ServerName :type String) (ServerMap :type String) (ServerMode :type String) (ServerSlots :type Integer))
  (Variables|Default|SetbShowMouseCursor true)
  (bind _returnvalue (UserInterface|CreateWidget "/Game/UI/Lobby.Lobby_C" 0 (Utilities|Text|ToText(String) ServerName) (Utilities|Text|ToText(String) ServerMap) (Utilities|Text|ToText(String) ServerMode) ServerSlots))
  (bind _output_get (Variables|Default|SetLobbyWB _returnvalue))
  (UserInterface|Viewport|AddtoViewport _output_get 1))

(event Custom|LoadingScreen
  (Widget|RemovefromParent (Variables|Default|GetLobbyWB))
  (bind _returnvalue (UserInterface|CreateWidget "/Game/UI/LoadingScreen.LoadingScreen_C" self))
  (UserInterface|Viewport|AddtoViewport _returnvalue 0))

(event Custom|GetChatMessage
  (params (SenderText :type Text))
  (Variables|Default|SetSenderText SenderText)
  (Variables|Default|SetSenderName (Class|AdvancedSessionsLibrary|GetPlayerName self))
  (bind _aslobby_game_mode (Utilities|Casting|CastToLobbyGameMode (Game|GetGameMode)))
  (for _array_element (Variables|/Game/BluePrints/LobbyGameMode.LobbyGameMode_C|GetAllPCs _aslobby_game_mode)
    (bind _aslobby_player_controller (Utilities|Casting|CastToLobbyPlayerController _array_element))
    (CallFunction|UpdateChat _aslobby_player_controller (Variables|Default|GetSenderName) (Variables|Default|GetSenderText))))

(event Custom|ClearPlayerList
  (Default|ClearPlayerList (Variables|Default|GetLobbyWB)))

(event Custom|AssignPlayer
  (params (Character :type BPX%20Player%20Class%20Reference)))

(event Custom|Kick
  (Game|OpenLevel(byName) "Menu")
  (|DestroySession self))

(event Custom|AddPlayer
  (params (Player :type Text) (PlayerIndex :type Integer))
  (Default|AddPlayertoList (Variables|Default|GetLobbyWB) Player PlayerIndex))

(event Custom|UpdateNumberofPlayers
  (params (CurrentPlayers :type Integer))
  (Variables|/Game/UI/Lobby.Lobby_C|SetCurrentPlayers (Variables|Default|GetLobbyWB) CurrentPlayers))

(event Custom|UpdateChat
  (params (Sender :type String) (Text :type Text))
  (Default|UpdateChatWindow (Variables|/Game/UI/Lobby.Lobby_C|GetChatWindow (Variables|Default|GetLobbyWB)) Sender Text))

(fn ConstructionScript)