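; Lobby game mode that manages connected players before a multiplayer match.
; Login and logout maintain a controller array; login also sends GameInstance server settings to the new player's lobby widget, and both rebuild every client's player list and count.
; It also kicks players by index, rebroadcasts collected player settings, and respawns and possesses chosen characters at the origin.
; JoinGame server-travels to the selected map, defaulting to NewMap.
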(event Custom|SwapCharacter
  (params (PlayerController :type Player%20Controller%20Object%20Reference) (CharacterClass :type BPX%20Player%20Class%20Reference) (ChangedStatus :type Boolean))
  (bind _returnvalue (Pawn|GetControlledPawn PlayerController))
  (if (not ChangedStatus)
    (Utilities|IsValid _returnvalue
      (:Is%20Valid
        (Actor|DestroyActor _returnvalue))
      (:Is%20Not%20Valid
        _))
    (bind _returnvalue_2 (Game|SpawnActorfromClass CharacterClass (Math|Transform|MakeTransform "0, 0, 0") "Undefined" 0 0))
    (Pawn|Possess PlayerController _returnvalue_2)))

(event Custom|UpdateServer
  (for _array_element (Variables|Default|GetAllPCs)
    (bind _aslobby_player_controller (Utilities|Casting|CastToLobbyPlayerController _array_element))
    (Default|ClearPlayerList _aslobby_player_controller)
    (for (_array_element_2 _array_index) (Variables|Default|GetAllPCs)
      (Default|AddPlayer _aslobby_player_controller (Utilities|Text|ToText(String) (Class|AdvancedSessionsLibrary|GetPlayerName _array_element_2)) _array_index)))
  (for _array_element_3 (Variables|Default|GetAllPCs)
    (bind _aslobby_player_controller_2 (Utilities|Casting|CastToLobbyPlayerController _array_element_3))
    (Default|UpdateNumberofPlayers _aslobby_player_controller_2 (Utilities|Array|Length (Variables|Default|GetAllPCs)))))

(event Custom|JoinGame
  (bind _returnvalue (Game|GetPlayerController 0))
  (if (Utilities|Enum|Equal(Enum) (Variables|Default|GetServerMap) "NewMap")
    (Development|ExecuteConsoleCommand "servertravel/Game/Maps/NewMap" _returnvalue :!label _label)
    (bind _asgame_instance_md9k (Utilities|Casting|CastToGameInstanceMD9K (Game|GetGameInstance)))
    (Default|JoinGame _asgame_instance_md9k)
    (elif (Utilities|Enum|Equal(Enum) (Variables|Default|GetServerMap) "MD9K_Test01")
      (Development|ExecuteConsoleCommand "servertravel/Game/Maps/MD9K_Test01" _returnvalue)
      (else
        (goto _label)))))

(event Custom|KickPlayer
  (params (Dimension%201 :type Integer))
  (bind _aslobby_player_controller (Utilities|Casting|CastToLobbyPlayerController (Utilities|Array|Get(acopy) (Variables|Default|GetAllPCs) Dimension%201)))
  (Default|Kick _aslobby_player_controller))

(event Custom|EveryoneUpdate
  (bind _allpcs (Variables|Default|GetAllPCs))
  (bind _output_get (Variables|Default|SetCurrentPlayers (Utilities|Array|Length (Variables|Default|GetAllPCs))))
  (if (> _output_get 0)
    (Utilities|Array|Clear (Variables|Default|GetConnectedPlayers))
    (for _array_element _allpcs
      (bind _aslobby_player_controller (Utilities|Casting|CastToLobbyPlayerController _array_element))
      (Utilities|Array|Add (Variables|Default|GetConnectedPlayers) (Variables|/Game/BluePrints/LobbyPlayerController.LobbyPlayerController_C|GetPlayerSettings _aslobby_player_controller)))
    (for _array_element_2 _allpcs
      (bind _aslobby_player_controller_2 (Utilities|Casting|CastToLobbyPlayerController _array_element_2))
      (Default|AddPlayerInfo _aslobby_player_controller_2 (Variables|Default|GetConnectedPlayers)))))

(event EventPostLogin
  (params (NewPlayer :type Player%20Controller%20Object%20Reference))
  (Networking|SwitchHasAuthority
    (:Authority
      (Utilities|Array|Add (Variables|Default|GetAllPCs) NewPlayer)
      (bind _asgame_instance_md9k (Utilities|Casting|CastToGameInstanceMD9K (Game|GetGameInstance)))
      (Variables|Default|SetServerName (Variables|/Game/BluePrints/GameInstanceMD9K.GameInstanceMD9K_C|GetServerName _asgame_instance_md9k))
      (Variables|Default|SetServerMap (Variables|/Game/BluePrints/GameInstanceMD9K.GameInstanceMD9K_C|GetServerMap _asgame_instance_md9k))
      (Variables|Default|SetServerMode (Variables|/Game/BluePrints/GameInstanceMD9K.GameInstanceMD9K_C|GetServerMode _asgame_instance_md9k))
      (Variables|Default|SetServerSlots (Variables|/Game/BluePrints/GameInstanceMD9K.GameInstanceMD9K_C|GetServerSlots _asgame_instance_md9k))
      (bind _aslobby_player_controller (Utilities|Casting|CastToLobbyPlayerController NewPlayer))
      (Default|InitialSetup _aslobby_player_controller)
      (Default|AddLobbyWB _aslobby_player_controller (Variables|Default|GetServerName) (Variables|Default|GetServerMap) (Variables|Default|GetServerMode) (Variables|Default|GetServerSlots))
      (CallFunction|UpdateServer))))

(event EventOnLogout
  (params (ExitingController :type Controller%20Object%20Reference))
  (bind _allpcs (Variables|Default|GetAllPCs))
  (bind (_array_element _array_index) (Utilities|Array|ForEachLoopwithBreak _allpcs :!label _label)
    (:LoopBody
      (if (== ExitingController _array_element)
        (goto _label Break)))
    (:Completed
      (Utilities|Array|RemoveIndex _allpcs _array_index)
      (CallFunction|UpdateServer))))

(fn ConstructionScript)