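; RedMinionPawn is a red minion creep pawn that tracks its spawn point and whether it stands in that spawn area.
; On BeginPlay it sets itself as the owning actor of its overhead health widget.
; Getters and setters, with the spawn-area setter called through an interface, expose the spawn state.
; When destroyed, it notifies its spawn point that the creep has died.
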(event EventBeginPlay
  (Utilities|IsValid self
    (:Is%20Valid
      (bind _ashealth_over_head (Utilities|Casting|CastToHealthOverHead (UserInterface|GetUserWidgetObject (Variables|Default|GetWidget))))
      (Variables|/Game/UI/HealthOverHead.HealthOverHead_C|SetOwningActor _ashealth_over_head self))))

(event EventDestroyed
  (Class|IMOBASpawner|CreepHasDied(Message) (Variables|Default|GetSpawnPointReference) self))

(fn ConstructionScript)

(fn GetIsCreepinSpawnArea
  (params (Is%20In%20Spawn%20Area :type Boolean))
  (return (Variables|Default|GetbCreepIsInSpawnPointArea)))

(fn SetIsCreepinSpawnArea
  (params (Is%20In%20Spawn%20Area :type Boolean))
  ;[0 0 0] Setter for the Spawn Area variable called through the Interface.
  (bind _output_get (Variables|Default|SetbCreepIsInSpawnPointArea Is%20In%20Spawn%20Area))
  (return _output_get))

(fn SetSpawnPoint
  (params (SpawnPointReference :type BP%20Lane%20Spawn%20Point%20Object%20Reference))
  (bind _output_get (Variables|Default|SetSpawnPointReference SpawnPointReference))
  (return _output_get))

(fn GetSpawnPoint
  (return (Variables|Default|GetSpawnPointReference)))